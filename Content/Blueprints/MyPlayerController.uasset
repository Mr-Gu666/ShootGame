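; Player controller that switches between a TP pawn (FirstPersonCharacter_BP) and an arms-only FP pawn while the left mouse button is held.
; Begin spawns both characters, TP at the player start and FP at a parking transform, then possesses TP.
; Pressing switches to FP and releasing returns to TP.
; Each swap moves the target pawn to the current pawn's transform, teleports the old one to the parking transform, then possesses the target.
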(event Custom|Begin
  (params (StartPoint :type Transform) (PlayerStart :type Transform))
  (Variables|Default|SetStartPoint StartPoint)
  (Variables|Default|SetPlayerStart PlayerStart)
  (bind _returnvalue (Game|SpawnActorfromClass "/Game/Blueprints/FirstPersonCharacter_BP.FirstPersonCharacter_BP_C" (Variables|Default|GetPlayerStart) "Undefined" 0 0))
  (Variables|Default|SetTP _returnvalue)
  (bind _returnvalue_2 (Game|SpawnActorfromClass "/Game/Blueprints/FPCharacter_OnlyArms_BP.FPCharacter_OnlyArms_BP_C" (Variables|Default|GetStartPoint) "Undefined" 0 0))
  (Variables|Default|SetFP _returnvalue_2)
  (Pawn|Possess (Variables|Default|GetTP)))

(event Custom|ChangeToFP
  (bind _returnvalue (Game|Player|GetPlayerPawn 0))
  (Transformation|SetActorTransform (Variables|Default|GetFP) (Transformation|GetActorTransform _returnvalue))
  (Transformation|SetActorTransform _returnvalue (Variables|Default|GetStartPoint))
  (Pawn|Possess (Variables|Default|GetFP)))

(event Custom|ChangeToTP
  (bind _returnvalue (Game|Player|GetPlayerPawn 0))
  (Transformation|SetActorTransform (Variables|Default|GetTP) (Transformation|GetActorTransform _returnvalue))
  (Transformation|SetActorTransform _returnvalue (Variables|Default|GetStartPoint))
  (Pawn|Possess (Variables|Default|GetTP)))

(event EventBeginPlay)

(event EventTick
  (params (DeltaSeconds :type Float%20%28single-precision%29)))

(event Input|MouseEvents|LeftMouseButton
  (params (Key :type Key%20Structure :default "None"))
  (:Pressed
    (CallFunction|ChangetoFP))
  (:Released
    (CallFunction|ChangetoTP)))

(fn ConstructionScript)